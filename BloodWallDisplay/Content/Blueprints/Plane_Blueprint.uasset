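; Plane actor that continuously rocks back and forth in pitch between two fixed rotations.
; On BeginPlay it stores the start and end rotators and plays a timeline that lerps the actor's rotation between them.
; When the timeline finishes, a boolean flag alternates between playing in reverse and from the start, creating an endless ping-pong motion.
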(event EventBeginPlay
  (Variables|Default|SetplaneRotState true)
  (Variables|Default|SetplaneStartRot (Math|Rotator|MakeRotator 0.0 7e+01 0.0))
  (Variables|Default|SetplaneDestRot (Math|Rotator|MakeRotator 0.0 9e+01 0.0))
  (bind _linear_0_to_1 (Timeline|Timeline_0 Play)
    (:Update
      (Transformation|SetActorRotation (Math|Rotator|Lerp(Rotator) (Variables|Default|GetplaneStartRot) (Variables|Default|GetplaneDestRot) _linear_0_to_1)))
    (:Finished
      (if (Variables|Default|GetplaneRotState)
        (Variables|Default|SetplaneRotState false)
        (Timeline|Timeline_0 ReverseFromEnd)
        (else
          (Variables|Default|SetplaneRotState true)
          (Timeline|Timeline_0 PlayFromStart))))))

(event Collision|EventActorBeginOverlap
  (params (OtherActor :type Actor%20Object%20Reference)))

(event EventTick
  (params (DeltaSeconds :type Float%20%28single-precision%29)))

(fn ConstructionScript)